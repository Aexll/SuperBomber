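; Movement component for player and bomb actors that moves them cell by cell on a grid in four directions.
; A looping timer glides the visual toward the cell edge, then the collision box jumps one cell and the visual shifts to the opposite edge, keeping motion smooth.
; Movement pauses at the cell centre, except when sliding, which continues until a box trace finds the next cell blocked.
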(event `self.ReceiveBeginPlay`
  (bind _returnvalue (`self.GetOwner`))
  (bind _x (.x (`BoxComponent.GetUnscaledBoxExtent` (`self.Box`))))
  (`|ExecutionSequence`
    (:`then_0`
      (bind _asbp_player_actor (cast `/Game/Blueprints/Actors/BP_PlayerActor` _returnvalue)
        (:`then`
          (set `self.Box` (`/Game/Blueprints/Actors/BP_PlayerActor.Box` _asbp_player_actor))
          (set `self.ToMove` (`/Game/Blueprints/Actors/BP_PlayerActor.Mesh` _asbp_player_actor)))
        (:`CastFailed`
          (bind _asbp_bombe (cast `/Game/Blueprints/Actors/BP_Bombe` _returnvalue))
          (set `self.Box` (`/Game/Blueprints/Actors/BP_Bombe.Box` _asbp_bombe))
          (set `self.ToMove` (`/Game/Blueprints/Actors/BP_Bombe.Scene` _asbp_bombe)))))
    (:`then_1`
      ;[1 0.4734 0] Init
      (set `self.Collisions` (`|MakeMap` "NewEnumerator0" false "NewEnumerator1" false "NewEnumerator2" false "NewEnumerator3" :!type "/Game/Blueprints/Enums/E_Direction Enum"))
      (bind _output_get (set `self.DirectionVectors` (`|MakeMap` "NewEnumerator0" (0.0 1.0 0.0) "NewEnumerator1" (0.0 -1.0 0.0) "NewEnumerator2" (-1.0 0.0 0.0) "NewEnumerator3" (1.0 0.0 0.0) :!type "/Game/Blueprints/Enums/E_Direction Enum" :!valuetype "Vector Structure")))
      (set `self.Pos` (`|MakeMap` "NewEnumerator0" (* _x (`BlueprintMapLibrary.Map_Find` _output_get "NewEnumerator0")) "NewEnumerator1" (* _x (`BlueprintMapLibrary.Map_Find` _output_get "NewEnumerator1")) "NewEnumerator2" (* _x (`BlueprintMapLibrary.Map_Find` _output_get "NewEnumerator2")) "NewEnumerator3" (* _x (`BlueprintMapLibrary.Map_Find` _output_get "NewEnumerator3")) "NewEnumerator4" :!type "/Game/Blueprints/Enums/E_Pos Enum")))))

(event `MoveTo`
  (params (Direction :type "/Game/Blueprints/Enums/E_Direction Enum" :default "NewEnumerator0") (Speed :type "Float (double-precision)"))
  (set `self.Speed` (* Speed 1.2))
  (set `self.MoveDirection` Direction)
  (if (`KismetSystemLibrary.K2_IsValidTimerHandle` (`self.Timer`))
    (`KismetSystemLibrary.K2_UnPauseTimerHandle` (`self.Timer`))
    (else
      (bind _returnvalue (`KismetSystemLibrary.K2_SetTimerDelegate` (delegate `MovementTick`) (`self.TimeDeltaTime`) true))
      (set `self.Timer` _returnvalue)
      (set `self.Moving` true))))

(event `MovementTick`
  (bind _currentmeshpos (`self.CurrentMeshPos`))
  ;[1 0.33 0] Move toward the direction
  (bind _output_get (set `self.CurrentMeshPos` (+ _currentmeshpos (* (`KismetMathLibrary.Normal` (- (`BlueprintMapLibrary.Map_Find` (`self.Pos`) (select `/Game/Blueprints/Enums/E_Direction` (`self.MoveDirection`) :`NewEnumerator0` "NewEnumerator0" :`NewEnumerator1` "NewEnumerator1" :`NewEnumerator2` "NewEnumerator2" :`NewEnumerator3` "NewEnumerator3" :`NewEnumerator4` "NewEnumerator4" :!type "/Game/Blueprints/Enums/E_Pos Enum")) _currentmeshpos)) (`self.TimeDeltaTime`) (`self.Speed`)))))
  (`SceneComponent.K2_SetRelativeLocation` (`self.ToMove`) _output_get false false)
  ;[1 0 0.33] Test if reached a box-transition position
  (if (== (`self.CurrentMeshPos`) (`BlueprintMapLibrary.Map_Find` (`self.Pos`) (select `/Game/Blueprints/Enums/E_Direction` (`self.MoveDirection`) :`NewEnumerator0` "NewEnumerator0" :`NewEnumerator1` "NewEnumerator1" :`NewEnumerator2` "NewEnumerator2" :`NewEnumerator3` "NewEnumerator3" :`NewEnumerator4` "NewEnumerator4" :!type "/Game/Blueprints/Enums/E_Pos Enum")) :`ErrorTolerance` (* (`self.TimeDeltaTime`) (`self.Speed`)))
    ;[0 0 1] Found
    (`self.MoveBox` (`self.MoveDirection`))
    (else
      ;[0 0 1] Not found
      (if (`self.Sliding`)
        ;[1 0 1] If mid stop
        (bind (_outhit _returnvalue) (`self.CalculateCollisionAtDirection` (`self.MoveDirection`)))
        (if _returnvalue
          (if (== (`self.CurrentMeshPos`) (`BlueprintMapLibrary.Map_Find` (`self.Pos`) "NewEnumerator4") :`ErrorTolerance` (* (`self.TimeDeltaTime`) (`self.Speed`))) :!label _label
            (`self.StopMovement`)))
        (else
          (goto _label))))))

(event `StopMovement`
  (`KismetSystemLibrary.K2_PauseTimerHandle` (`self.Timer`))
  (set `self.Moving` false))

(fn `CalculateCollisionAtDirection`
  (params (Direction :type "/Game/Blueprints/Enums/E_Direction Enum (by ref)"))
  (returns (OutHit :type "HitResult Structure") (ReturnValue :type Boolean))
  (bind _returnvalue (+ (`SceneComponent.K2_GetComponentLocation` (`self.Box`)) (* (`BlueprintMapLibrary.Map_Find` (`self.DirectionVectors`) Direction) (.x (`BoxComponent.GetUnscaledBoxExtent` (`self.Box`))) 2.0)))
  (bind (_outhit _returnvalue_2) (`KismetSystemLibrary.BoxTraceSingle` _returnvalue _returnvalue (45.0 45.0 45.0) (struct) "TraceTypeQuery1" false (`|MakeArray` (`self.GetOwner`)) "None" true (struct :`R` 0.106753 :`B` 1.0 :`A` 1.0) (struct :`R` 0.863357 :`B` 1.0 :`A` 1.0) 0.1))
  (return _outhit _returnvalue_2))

(fn `MoveBox`
  (params (MovingDirection :type "/Game/Blueprints/Enums/E_Direction Enum" :default "NewEnumerator0"))
  (bind _value (`BlueprintMapLibrary.Map_Find` (`self.Pos`) (select `/Game/Blueprints/Enums/E_Direction` (`local.MovingDirection`) :`NewEnumerator0` "NewEnumerator1" :`NewEnumerator1` "NewEnumerator0" :`NewEnumerator2` "NewEnumerator3" :`NewEnumerator3` "NewEnumerator2" :`NewEnumerator4` "NewEnumerator4" :!type "/Game/Blueprints/Enums/E_Pos Enum")))
  ;[0 0 1] Move the box
  (`SceneComponent.K2_AddWorldOffset` (`self.Box`) (* (`BlueprintMapLibrary.Map_Find` (`self.DirectionVectors`) MovingDirection) (.x (`BoxComponent.GetUnscaledBoxExtent` (`self.Box`))) 2.0) false false)
  ;[1 0.5 0] Move mesh to the oposite relative location
  (bind _output_get (set `self.CurrentMeshPos` (- _value (* (`KismetMathLibrary.Normal` _value) (* (`self.TimeDeltaTime`) (`self.Speed`))))))
  (`SceneComponent.K2_SetRelativeLocation` (`self.ToMove`) _output_get false false))