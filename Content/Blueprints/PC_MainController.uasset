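; PC_MainController is the player controller that creates and shows the game's HUD screens.
; On BeginPlay it creates the main HUD widget and adds it to the viewport.
; Custom events add a waiting-to-start screen and an end screen that receives whether the player won, keeping a reference to each widget.
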(event `self.ReceiveBeginPlay`
  (bind _returnvalue (`|CreateWidget` "/Game/HUD/HUD_MainWidget.HUD_MainWidget_C" self))
  (bind _output_get (set `self.HUD_Main` _returnvalue))
  (`UserWidget.AddToViewport` _output_get 0))

(event `/Game/Blueprints/Interfaces/I_GameState.GameEnd`
  (params (PlayerWon :type "/Game/Blueprints/Actors/BP_PlayerActor Object Reference"))
  (bind _returnvalue (`|CreateWidget` "/Game/HUD/HUD_GameEnd.HUD_GameEnd_C" self PlayerWon))
  (bind _output_get (set `self.HUD_End` _returnvalue))
  (`UserWidget.AddToViewport` _output_get 0))

(event `/Game/Blueprints/Interfaces/I_GameState.GameWaitToStart`
  (bind _returnvalue (`|CreateWidget` "/Game/HUD/HUD_GameWaitingToStart.HUD_GameWaitingToStart_C" self))
  (bind _output_get (set `self.HUD_GameWaiting` _returnvalue))
  (`UserWidget.AddToViewport` _output_get 0))

(fn `UserConstructionScript`)