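; Player actor for a Bomberman-style grid game, with per-player color and keys, bonus-scaled bombs and speed, weapon switching, health, invincibility, freezing and respawn.
; An input stack picks the latest direction not blocked by box traces, and pushable actors in that direction receive a push message.
; A looping timer slides the mesh toward the cell edge, then jumps the collision box one cell and re-offsets the mesh for continuous-looking movement.
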(event `self.ReceiveBeginPlay`
  (bind _playerindex (`self.PlayerIndex`))
  (bind _playerindex_2 (`self.PlayerIndex`))
  (bind _playersinputs (`/Game/Blueprints/GI.PlayersInputs` (`self.GI`)))
  (bind _x (.x (`BoxComponent.GetUnscaledBoxExtent` (`self.Box`))))
  ;[1 0.57 0] Init
  ;;[1 0.08854 0.08854] Binds
  (add `self.GetBonus` (delegate `GetBonus_Event`))
  (add `self.Respawn` (delegate `Revive`))
  (set `self.Collisions` (`|MakeMap` "NewEnumerator0" false "NewEnumerator1" false "NewEnumerator2" false "NewEnumerator3" :!type "/Game/Blueprints/Enums/E_Direction Enum"))
  (bind _output_get (set `self.DirectionVectors` (`|MakeMap` "NewEnumerator0" (0.0 1.0 0.0) "NewEnumerator1" (0.0 -1.0 0.0) "NewEnumerator2" (-1.0 0.0 0.0) "NewEnumerator3" (1.0 0.0 0.0) :!type "/Game/Blueprints/Enums/E_Direction Enum" :!valuetype "Vector Structure")))
  (set `self.Pos` (`|MakeMap` "NewEnumerator0" (* _x (`BlueprintMapLibrary.Map_Find` _output_get "NewEnumerator0")) "NewEnumerator1" (* _x (`BlueprintMapLibrary.Map_Find` _output_get "NewEnumerator1")) "NewEnumerator2" (* _x (`BlueprintMapLibrary.Map_Find` _output_get "NewEnumerator2")) "NewEnumerator3" (* _x (`BlueprintMapLibrary.Map_Find` _output_get "NewEnumerator3")) "NewEnumerator4" :!type "/Game/Blueprints/Enums/E_Pos Enum"))
  (for _array_element (`|MakeArray` "NewEnumerator0" "NewEnumerator1" "NewEnumerator3" "NewEnumerator2" :!type "/Game/Blueprints/Enums/E_Bonus Enum")
    (`BlueprintMapLibrary.Map_Add` (`self.Bonus`) _array_element))
  (bind _asgm (cast `/Game/Blueprints/GM` (`GameplayStatics.GetGameMode`)))
  (set `self.GM` _asgm)
  (bind _asgi (cast `/Game/Blueprints/GI` (`GameplayStatics.GetGameInstance`)))
  (bind _output_get_2 (set `self.GI` _asgi))
  (bind _playerscolors (`/Game/Blueprints/GI.PlayersColors` _output_get_2))
  ;;[0 0 1] Player color
  (set `self.PlayerColor` (select `bool` (`KismetArrayLibrary.Array_IsValidIndex` _playerscolors _playerindex_2) :`false` (`KismetMathLibrary.Conv_LinearColorToColor` (`KismetMathLibrary.HSVToRGB` (`KismetMathLibrary.RandomFloatInRange` 0.0 360.0) 0.75 1.0)) :`true` (`|GetArrayItem` _playerscolors _playerindex_2)))
  ;;[0 1 0] Player material
  (bind _returnvalue (`PrimitiveComponent.CreateDynamicMaterialInstance` (`self.Mesh`) 0 "/Game/Materials/M_Player.M_Player" "None"))
  (bind _output_get_3 (set `self.DynamicMaterial` _returnvalue))
  (`MaterialInstanceDynamic.SetVectorParameterValue` _output_get_3 "Color" (`KismetMathLibrary.Conv_ColorToLinearColor` (`self.PlayerColor`)))
  ;;[1 0 1] Player name
  (set `self.PlayerName` (`KismetStringLibrary.Concat_StrStr` "Player " (`KismetStringLibrary.Conv_IntToString` (+ (`self.PlayerIndex`) 1))))
  ;;[1 0.09375 0.09375] Set input
  (if (`KismetArrayLibrary.Array_IsValidIndex` _playersinputs _playerindex)
    (set `self.Inputs` (`.Input_34_A3CDC1BE417761C73C8CE7A15C1603C8` (break `/Game/Blueprints/Structure/S_GlobalPlayeInput` (`|GetArrayItem` _playersinputs _playerindex))))
    (else
      (set `self.Inputs` (`.Input_34_A3CDC1BE417761C73C8CE7A15C1603C8` (break `/Game/Blueprints/Structure/S_GlobalPlayeInput` (`/Game/Blueprints/GI.DefaultPlayerInput` (`self.GI`))))))))

(event `GetBonus_Event` :!signature `self.GetBonus`
  (params (Bonus :type "/Game/Blueprints/Enums/E_Bonus Enum" :default "NewEnumerator0") (NB :type Integer))
  ;[1 0.57 0] Init
  ;;[1 0.08854 0.08854] Binds
  ;;;[0 0.4635 0.04682] Get bonus
  (`BlueprintMapLibrary.Map_Add` (`self.Bonus`) Bonus (+ (`BlueprintMapLibrary.Map_Find` (`self.Bonus`) Bonus) NB)))

(event `self.ReceiveTick`
  (params (DeltaSeconds :type "Float (single-precision)"))
  ;[1 0 1] Tick
  (if (`self.ActiveInput`)
    (`self.CalculateAllCollisions`)
    (bind (_input _validinput) (`self.GetFirstValidDirectionFromStack`))
    (if _validinput
      (`self.MoveTo` _input)
      (bind (_outhit _returnvalue) (`self.CalculateCollisionAtDirection` _input))
      (if _returnvalue
        (message `/Game/Blueprints/Interfaces/I_GameInteractions.Pushed` (`.HitActor` (`GameplayStatics.BreakHitResult` _outhit)) _input (`self.SpeedByBonus`))))))

(event `MoveTo`
  (params (Direction :type "/Game/Blueprints/Enums/E_Direction Enum" :default "NewEnumerator0"))
  ;[0 0 1] Timer
  (set `self.MoveDirection` Direction)
  (if (`KismetSystemLibrary.K2_IsValidTimerHandle` (`self.Timer`))
    (`KismetSystemLibrary.K2_UnPauseTimerHandle` (`self.Timer`))
    (else
      (bind _returnvalue (`KismetSystemLibrary.K2_SetTimerDelegate` (delegate `MovementTick`) (`self.TimeDeltaTime`) true))
      (set `self.Timer` _returnvalue))))

(event `MovementTick`
  (bind _currentmeshpos (`self.CurrentMeshPos`))
  ;[1 0.33 0] Move toward the direction
  (`SceneComponent.K2_SetRelativeLocation` (`self.NextEmplacement`) (* (`BlueprintMapLibrary.Map_Find` (`self.DirectionVectors`) (`self.MoveDirection`)) 100) false false)
  (bind _output_get (set `self.CurrentMeshPos` (+ _currentmeshpos (* (`KismetMathLibrary.Normal` (- (`BlueprintMapLibrary.Map_Find` (`self.Pos`) (select `/Game/Blueprints/Enums/E_Direction` (`self.MoveDirection`) :`NewEnumerator0` "NewEnumerator0" :`NewEnumerator1` "NewEnumerator1" :`NewEnumerator2` "NewEnumerator2" :`NewEnumerator3` "NewEnumerator3" :`NewEnumerator4` "NewEnumerator4" :!type "/Game/Blueprints/Enums/E_Pos Enum")) _currentmeshpos)) (`self.TimeDeltaTime`) (`self.SpeedByBonus`)))))
  (`SceneComponent.K2_SetRelativeLocation` (`self.Mesh`) _output_get false false)
  ;[1 0 0.33] Test if reached a box-transition position
  (if (== (`self.CurrentMeshPos`) (`BlueprintMapLibrary.Map_Find` (`self.Pos`) (select `/Game/Blueprints/Enums/E_Direction` (`self.MoveDirection`) :`NewEnumerator0` "NewEnumerator0" :`NewEnumerator1` "NewEnumerator1" :`NewEnumerator2` "NewEnumerator2" :`NewEnumerator3` "NewEnumerator3" :`NewEnumerator4` "NewEnumerator4" :!type "/Game/Blueprints/Enums/E_Pos Enum")) :`ErrorTolerance` (* (`self.TimeDeltaTime`) (`self.Speed`)))
    ;[0 0 1] Found
    (`self.MoveBox` (`self.MoveDirection`))
    (else
      ;[0 0 1] Not found
      (if (== (`self.CurrentMeshPos`) (`BlueprintMapLibrary.Map_Find` (`self.Pos`) "NewEnumerator4") :`ErrorTolerance` (* (`self.TimeDeltaTime`) (`self.Speed`)))
        (bind (_input _validinput) (`self.GetFirstValidDirectionFromStack`))
        (if (not _validinput)
          (`KismetSystemLibrary.K2_PauseTimerHandle` (`self.Timer`))
          (`SceneComponent.K2_SetRelativeLocation` (`self.NextEmplacement`) (0.0 0.0 0.0) false false))))))

(event `Action_1`
  (bind _returnvalue (`SceneComponent.K2_GetComponentLocation` (`self.Box`)))
  ;[1 0 0] Actions Input
  (if (`self.ActiveInput`)
    (if (< (`self.BombeCount`) (+ (`BlueprintMapLibrary.Map_Find` (`self.Bonus`) "NewEnumerator3") 1))
      ;;[1 0.25 0.25] Test if bomb are overlaping
      (bind (_outhit _returnvalue_2) (`KismetSystemLibrary.LineTraceSingleForObjects` (+ _returnvalue (0.0 0.0 45.0)) (+ _returnvalue (0.0 0.0 -45.0)) (`|MakeArray` "ObjectTypeQuery9" :!type "EObjectTypeQuery Enum")))
      (if (not _returnvalue_2)
        ;;[0.003 0 0.18] Spawn bombe
        (bind _returnvalue_3 (`|SpawnActorFromClass` (`self.CurrentWeapon`) (`KismetMathLibrary.MakeTransform` (`self.K2_GetActorLocation`)) "Undefined" "OverrideRootScale" null self null))
        (bind _bonuses (`/Game/Blueprints/Actors/BP_Bombe.Bonuses` _returnvalue_3))
        (`BlueprintMapLibrary.Map_Add` _bonuses "NewEnumerator0" (+ (`BlueprintMapLibrary.Map_Find` (`self.Bonus`) "NewEnumerator0") 1))
        (`BlueprintMapLibrary.Map_Add` _bonuses "NewEnumerator1" (`BlueprintMapLibrary.Map_Find` (`self.Bonus`) "NewEnumerator1"))))))

(event `Action_2`
  ;[1 0 0] Actions Input
  (if (`self.ActiveInput`)
    (`/Engine/EditorBlueprintResources/StandardMacros.FlipFlop`
      (:`A`
        (`self.ChangeWeapon` "/Game/Blueprints/Actors/Bombes/BP_Bombe_Quantum.BP_Bombe_Quantum_C"))
      (:`B`
        (`self.ChangeWeapon` "/Game/Blueprints/Actors/Bombes/BP_Bombe_Ice.BP_Bombe_Ice_C")))))

(event `/Game/Blueprints/Interfaces/I_GameInteractions.Blowed`
  (params (Damages :type Integer) (Direction :type "Vector Structure"))
  (`self.Damaged` Damages))

(event `Damaged`
  (params (Damages :type Integer))
  ;[1 0.06667 0] Damaged
  (if (not (`self.Invincible`))
    (bind _output_get (set `self.Health` (- (`self.Health`) Damages)))
    (if (> _output_get 0)
      (`KismetSystemLibrary.K2_SetTimerDelegate` (delegate `RemoveUnvulnerability`) (`self.InvincibilityTime`))
      (`MaterialInstanceDynamic.SetScalarParameterValue` (`self.DynamicMaterial`) "Invincible" 1.0)
      (set `self.Invincible` true)
      (else
        (`self.Die`)))))

(event `RemoveUnvulnerability`
  ;[1 0 0.6667] Invulnerability
  (set `self.Invincible` false)
  (`MaterialInstanceDynamic.SetScalarParameterValue` (`self.DynamicMaterial`) "Invincible" 0.0))

(event `Die`
  (bind _box (`self.Box`))
  ;[1 0 0] Die
  (if (`self.Alive`)
    (set `self.ActiveInput` false)
    (set `self.Alive` false)
    (`SceneComponent.SetVisibility` _box false true)
    (`PrimitiveComponent.SetCollisionEnabled` _box "NoCollision")
    (`PrimitiveComponent.SetCollisionEnabled` (`self.NextEmplacement`) "NoCollision")
    (bind _returnvalue (`NiagaraFunctionLibrary.SpawnSystemAtLocation` "/Game/Particle/P_PlayerDie.P_PlayerDie" (`SceneComponent.K2_GetComponentLocation` (`self.Box`))))
    (`FXSystemComponent.SetColorParameter` _returnvalue "Color" (`KismetMathLibrary.Conv_ColorToLinearColor` (`self.PlayerColor`)))
    ;;[1 0.5299 0.2292] Message
    (bind _outactors (`GameplayStatics.GetAllActorsWithInterface` "/Game/Blueprints/Interfaces/I_GameInteractions.I_GameInteractions_C"))
    (for _array_element _outactors
      (message `/Game/Blueprints/Interfaces/I_GameInteractions.PlayerDied` _array_element self))))

(event `Revive`
  (bind _box (`self.Box`))
  ;[0 1 0] Revive
  (set `self.Health` (`self.MaxHealth`))
  (set `self.Invincible` false)
  (set `self.ActiveInput` true)
  (set `self.Alive` true)
  (`SceneComponent.SetVisibility` _box true true)
  (`PrimitiveComponent.SetCollisionEnabled` _box "QueryAndPhysics")
  (`PrimitiveComponent.SetCollisionEnabled` (`self.NextEmplacement`) "QueryAndPhysics")
  (for _array_element (`|MakeArray` "NewEnumerator0" "NewEnumerator1" "NewEnumerator3" "NewEnumerator2" :!type "/Game/Blueprints/Enums/E_Bonus Enum")
    (`BlueprintMapLibrary.Map_Add` (`self.Bonus`) _array_element)))

(event `/Game/Blueprints/Interfaces/I_GameState.GameStart`
  ;[1 0.35 0] GameState
  (`self.Respawn`)
  (`self.ChangeWeapon` "/Game/Blueprints/Actors/Bombes/BP_Bombe_Classique.BP_Bombe_Classique_C"))

(event `/Game/Blueprints/Interfaces/I_GameState.GameEnd`
  (params (PlayerWon :type "/Game/Blueprints/Actors/BP_PlayerActor Object Reference"))
  ;[1 0.35 0] GameState
  (`KismetArrayLibrary.Array_Clear` (`self.InputStack`))
  (set `self.Invincible` true)
  (set `self.ActiveInput` false))

(event `/Game/Blueprints/Interfaces/I_GameInteractions.PlayerDied`
  (params (Player :type "/Game/Blueprints/Actors/BP_PlayerActor Object Reference")))

(event `ChangeWeapon`
  (params (CurrentWeapon :type "/Game/Blueprints/Actors/BP_Bombe Class Reference"))
  (set `self.CurrentWeapon` CurrentWeapon)
  ;[0 0 1] change weapon in widget
  (bind _hud (`self.HUD`)
    (:`then`
      (`/Game/HUD/HUD_PlayerState.ChangeWeapon` _hud)
      (bind _ashud_switch_bombe (cast `/Game/HUD/HUD_SwitchBombe` (`WidgetComponent.GetWidget` (`self.Widget`))))
      (`UserWidget.PlayAnimation` _ashud_switch_bombe (`/Game/HUD/HUD_SwitchBombe.Switch` _ashud_switch_bombe) 0.0 1 "Forward" 1.0 false)
      (`/Game/HUD/HUD_SwitchBombe.SetImage` _ashud_switch_bombe (`self.CurrentWeapon`)))
    (:`else`)))

(event `/Game/Blueprints/Interfaces/I_GameInteractions.Freezed`
  (params (Level :type Integer))
  (bind _timer (`self.Timer`))
  ;[0 0.5 1] Freezed
  (if (not (`self.IsFreezed`))
    (set `self.IsFreezed` true)
    (set `self.ActiveInput` false)
    (bind _returnvalue (`NiagaraFunctionLibrary.SpawnSystemAtLocation` "/Game/Particle/P_Freezed.P_Freezed" (`SceneComponent.K2_GetComponentLocation` (`self.Mesh`))))
    (set `self.FrozeTimer` (`KismetSystemLibrary.K2_IsTimerActiveHandle` _timer))
    (`KismetSystemLibrary.K2_PauseTimerHandle` _timer))
  (`KismetSystemLibrary.RetriggerableDelay` (* (`KismetMathLibrary.Conv_IntToDouble` Level) 1.0))
  (set `self.IsFreezed` false)
  (if (`self.FrozeTimer`)
    (`KismetSystemLibrary.K2_UnPauseTimerHandle` _timer))
  (`ActorComponent.K2_DestroyComponent` _returnvalue)
  (if (`|EnumEquality` (`/Game/Blueprints/GM.State` (`self.GM`)) "NewEnumerator0")
    (set `self.ActiveInput` true)))

(fn `CalculateAllCollisions`
  (for _array_element (`|MakeArray` "NewEnumerator0" "NewEnumerator1" "NewEnumerator2" "NewEnumerator3" :!type "/Game/Blueprints/Enums/E_Direction Enum")
    (bind (_outhit _returnvalue) (`self.CalculateCollisionAtDirection` _array_element))
    (bind (_bblockinghit _binitialoverlap _time _distance _location _impactpoint _normal _impactnormal _physmat _hitactor) (`GameplayStatics.BreakHitResult` _outhit))
    (if (`KismetSystemLibrary.DoesImplementInterface` _hitactor "/Game/Blueprints/Interfaces/I_GameInteractions.I_GameInteractions_C")
      (bind _pushable (message `/Game/Blueprints/Interfaces/I_GameInteractions.Pushable` _hitactor _array_element))
      (if _pushable
        (`BlueprintMapLibrary.Map_Add` (`self.Collisions`) _array_element)
        (else
          (`BlueprintMapLibrary.Map_Add` (`self.Collisions`) _array_element _returnvalue :!label _label)))
      (else
        (goto _label))))
  (return))

(fn `CalculateCollisionAtDirection`
  (params (Direction :type "/Game/Blueprints/Enums/E_Direction Enum (by ref)"))
  (returns (OutHit :type "HitResult Structure") (ReturnValue :type Boolean))
  (bind _returnvalue (+ (`SceneComponent.K2_GetComponentLocation` (`self.Box`)) (* (`BlueprintMapLibrary.Map_Find` (`self.DirectionVectors`) Direction) (.x (`BoxComponent.GetUnscaledBoxExtent` (`self.Box`))) 2.0)))
  (bind (_outhit _returnvalue_2) (`KismetSystemLibrary.BoxTraceSingle` _returnvalue _returnvalue (45.0 45.0 45.0) (struct) "TraceTypeQuery1" false (`|MakeArray` self :!type "Actor Object Reference") (select `bool` false :`true` "ForDuration" :!type "EDrawDebugTrace Enum") true (struct :`R` 0.106753 :`B` 1.0 :`A` 1.0) (struct :`R` 0.863357 :`B` 1.0 :`A` 1.0) 0.1))
  (return _outhit _returnvalue_2))

(fn `GetFirstValidDirectionFromStack`
  (returns (Input :type "/Game/Blueprints/Enums/E_Direction Enum") (ValidInput :type Boolean))
  (if (`KismetMathLibrary.Conv_IntToBool` (`KismetArrayLibrary.Array_Length` (`self.InputStack`)))
    (bind (_arrayindex _arrayelement) (`/Engine/EditorBlueprintResources/StandardMacros.ReverseForEachLoop` (`self.InputStack`))
      (:`LoopBody`
        (if (not (`BlueprintMapLibrary.Map_Find` (`self.Collisions`) _arrayelement))
          (return _arrayelement true)))
      (:`Completed`
        (return "NewEnumerator4" false)))
    (else
      (return "NewEnumerator4" false))))

(fn `Input_Pressed`
  (params (Key :type "Key Structure" :default "None"))
  (bind _inputs (`self.Inputs`))
  (bind _values (`BlueprintMapLibrary.Map_Values` _inputs))
  (bind _returnvalue (`KismetArrayLibrary.Array_Find` _values Key))
  (if (!= _returnvalue -1)
    (bind _keys (`BlueprintMapLibrary.Map_Keys` _inputs))
    (switch `/Game/Blueprints/Enums/E_InputAction` (`|GetArrayItem` _keys _returnvalue)
      (:`NewEnumerator0`
        (`KismetArrayLibrary.Array_Add` (`self.InputStack`) "NewEnumerator0"))
      (:`NewEnumerator1`
        (`KismetArrayLibrary.Array_Add` (`self.InputStack`) "NewEnumerator1"))
      (:`NewEnumerator2`
        (`KismetArrayLibrary.Array_Add` (`self.InputStack`) "NewEnumerator2"))
      (:`NewEnumerator3`
        (`KismetArrayLibrary.Array_Add` (`self.InputStack`) "NewEnumerator3"))
      (:`NewEnumerator4`
        (`self.Action_1`))
      (:`NewEnumerator5`
        (`self.Action_2`)))))

(fn `Input_Release`
  (params (Key :type "Key Structure" :default "None"))
  (bind _inputs (`self.Inputs`))
  (bind _values (`BlueprintMapLibrary.Map_Values` _inputs))
  (bind _returnvalue (`KismetArrayLibrary.Array_Find` _values Key))
  (if (!= _returnvalue -1)
    (bind _keys (`BlueprintMapLibrary.Map_Keys` _inputs))
    (switch `/Game/Blueprints/Enums/E_InputAction` (`|GetArrayItem` _keys _returnvalue)
      (:`NewEnumerator0`
        (`KismetArrayLibrary.Array_RemoveItem` (`self.InputStack`) "NewEnumerator0"))
      (:`NewEnumerator1`
        (`KismetArrayLibrary.Array_RemoveItem` (`self.InputStack`) "NewEnumerator1"))
      (:`NewEnumerator2`
        (`KismetArrayLibrary.Array_RemoveItem` (`self.InputStack`) "NewEnumerator2"))
      (:`NewEnumerator3`
        (`KismetArrayLibrary.Array_RemoveItem` (`self.InputStack`) "NewEnumerator3")))))

(fn `MoveBox`
  (params (MovingDirection :type "/Game/Blueprints/Enums/E_Direction Enum" :default "NewEnumerator0"))
  (bind _value (`BlueprintMapLibrary.Map_Find` (`self.Pos`) (select `/Game/Blueprints/Enums/E_Direction` (`local.MovingDirection`) :`NewEnumerator0` "NewEnumerator1" :`NewEnumerator1` "NewEnumerator0" :`NewEnumerator2` "NewEnumerator3" :`NewEnumerator3` "NewEnumerator2" :`NewEnumerator4` "NewEnumerator4" :!type "/Game/Blueprints/Enums/E_Pos Enum")))
  (`SceneComponent.K2_AddWorldOffset` (`self.Box`) (* (`BlueprintMapLibrary.Map_Find` (`self.DirectionVectors`) MovingDirection) (.x (`BoxComponent.GetUnscaledBoxExtent` (`self.Box`))) 2.0) false false)
  (bind _output_get (set `self.CurrentMeshPos` (- _value (* (`KismetMathLibrary.Normal` _value) 1.0))))
  (`SceneComponent.K2_SetRelativeLocation` (`self.Mesh`) _output_get false false)
  (`self.CalculateAllCollisions`))

(fn `Pushable`
  (params (Direction :type "/Game/Blueprints/Enums/E_Direction Enum" :default "NewEnumerator0"))
  (returns (Pushable :type Boolean))
  (return false))

(fn `SpeedByBonus`
  (returns (ReturnValue :type "Float (double-precision)"))
  (return (+ (`self.Speed`) (`KismetMathLibrary.FClamp` (* (`BlueprintMapLibrary.Map_Find` (`self.Bonus`) "NewEnumerator2") 50) 0.0 500.0))))

(fn `UserConstructionScript`
  (`SceneComponent.SetHiddenInGame` (`self.Box`) (not (`self.Debug`)) false)
  (`SceneComponent.SetHiddenInGame` (`self.RIGHT`) (not (`self.Debug`)) false)
  (`SceneComponent.SetHiddenInGame` (`self.UP`) (not (`self.Debug`)) false))