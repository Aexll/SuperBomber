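; Quantum bomb variant that randomly teleports across the map grid until it detonates, triggering itself on BeginPlay.
; Tick uses a bonus-scaled Delay to attempt jumps to random grid-snapped points within a bonus-sized area, moving only if the spot is valid and clear.
; Detonate traces four directions with bonus-based reach, spawns sized Niagara blasts, sends BlowedMessage to interface actors at the collected positions, then destroys the bomb.
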(event `self.ReceiveBeginPlay`
  (`parent.ReceiveBeginPlay`)
  (`self.Trigger`))

(event `Teleport`
  (bind _returnvalue (`SceneComponent.K2_GetComponentLocation` (`self.Box`)))
  (bind _returnvalue_2 (`KismetMathLibrary.Conv_IntToDouble` (* (+ (`BlueprintMapLibrary.Map_Find` (`self.Bonuses`) "NewEnumerator0") 0) 100)))
  (bind _output_get (set `self.ToTeleport` (`KismetMathLibrary.MakeVector` (.x (`KismetMathLibrary.Vector_SnappedToGrid` (`KismetMathLibrary.RandomPointInBoundingBox` _returnvalue (`KismetMathLibrary.MakeVector` _returnvalue_2 _returnvalue_2)) 100.0)) (.y (`KismetMathLibrary.Vector_SnappedToGrid` (`KismetMathLibrary.RandomPointInBoundingBox` _returnvalue (`KismetMathLibrary.MakeVector` _returnvalue_2 _returnvalue_2)) 100.0)) (.z _returnvalue))))
  (bind _valide (`/Game/Blueprints/CollisionsFunctions.PositionInMap` _output_get))
  (if _valide
    (bind (_outhits _returnvalue_3) (`/Game/Blueprints/CollisionsFunctions.PositionTest` _output_get "TraceTypeQuery3"))
    (if (not _returnvalue_3)
      (`NiagaraFunctionLibrary.SpawnSystemAtLocation` "/Game/Particle/QuantumBombe/P_QuantumTeleport.P_QuantumTeleport" (`SceneComponent.K2_GetComponentLocation` (`self.Box`)) (struct) (`SceneComponent.RelativeScale3D` (`self.Sphere`)))
      (`self.K2_SetActorLocation` (`self.ToTeleport`)))))

(event `self.ReceiveTick`
  (params (DeltaSeconds :type "Float (single-precision)"))
  (`parent.ReceiveTick` DeltaSeconds)
  (`KismetSystemLibrary.Delay` (/ 0.5 (+ (`BlueprintMapLibrary.Map_Find` (`self.Bonuses`) "NewEnumerator1") 1)))
  (`self.Teleport`))

(event `self.Detonate`
  (`parent.Detonate`)
  (`|ExecutionSequence`
    (:`then_0`
      ;[1 0.3901 0] GetLocations
      (for _array_element (`|MakeArray` "NewEnumerator0" "NewEnumerator1" "NewEnumerator2" "NewEnumerator3" :!type "/Game/Blueprints/Enums/E_Direction Enum")
        (bind (_vallidpos1 _collidpos1 _size) (`/Game/Blueprints/CollisionsFunctions.DirectionTillHit` (`self.Box`) (`BlueprintMapLibrary.Map_Find` (`self.DirectionsVectors`) _array_element) (* (`BlueprintMapLibrary.Map_Find` (`self.Bonuses`) "NewEnumerator0") 1)))
        (bind _result (`BlueprintSetLibrary.Set_Union` (`self.ToDamagePos`) _vallidpos1))
        (set `self.ToDamagePos` _result)
        (bind _result_2 (`BlueprintSetLibrary.Set_Union` (`self.ToBreakPos`) _collidpos1))
        (set `self.ToBreakPos` _result_2)
        ;[1 0 1] Particles
        (bind _returnvalue (`NiagaraFunctionLibrary.SpawnSystemAtLocation` "/Game/Particle/QuantumBombe/P_QuantumExplosion.P_QuantumExplosion" (`SceneComponent.K2_GetComponentLocation` (`self.Box`)) (`BlueprintMapLibrary.Map_Find` (`self.DirectionsRotators`) _array_element)))
        (`FXSystemComponent.SetIntParameter` _returnvalue "Size" _size))
      ;[0.9896 0.1519 0] Blow
      (bind _result_3 (`BlueprintSetLibrary.Set_Union` (`self.ToBreakPos`) (`self.ToDamagePos`)))
      (bind _result_4 (`BlueprintSetLibrary.Set_ToArray` _result_3))
      (for _array_element_2 _result_4
        (bind _outhits (`/Game/Blueprints/CollisionsFunctions.PositionTest` _array_element_2))
        (for _array_element_3 _outhits
          (bind (_bblockinghit _binitialoverlap _time _distance _location _impactpoint _normal _impactnormal _physmat _hitactor) (`GameplayStatics.BreakHitResult` _array_element_3))
          (if (`KismetSystemLibrary.DoesImplementInterface` _hitactor "/Game/Blueprints/Interfaces/I_GameInteractions.I_GameInteractions_C")
            (message `/Game/Blueprints/Interfaces/I_GameInteractions.Blowed` _hitactor (`self.Damages`) (`KismetMathLibrary.Normal` (- _array_element_2 (`SceneComponent.K2_GetComponentLocation` (`self.Box`)))))))))
    (:`then_1`
      (`self.K2_DestroyActor`))))

(fn `UserConstructionScript`
  (`parent.UserConstructionScript`))