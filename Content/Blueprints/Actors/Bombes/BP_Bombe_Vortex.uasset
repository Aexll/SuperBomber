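; Vortex bomb variant that triggers itself on BeginPlay and, on detonation, blasts along four directions before destroying itself.
; Each direction's reach comes from a bonus value and a one-hit check, which collects damage and break positions and sizes an explosion effect.
; Actors found at those positions receive BlowedMessage through I_GameInteractions, with damage and an outward direction.
; A crate-spawning branch is left disconnected.
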(event `self.ReceiveBeginPlay`
  (`parent.ReceiveBeginPlay`)
  (`self.Trigger`))

(event `self.Detonate`
  (`parent.Detonate`)
  (`|ExecutionSequence`
    (:`then_0`
      ;[1 0.3901 0] GetLocations
      (for _array_element (`|MakeArray` "NewEnumerator0" "NewEnumerator1" "NewEnumerator2" "NewEnumerator3" :!type "/Game/Blueprints/Enums/E_Direction Enum")
        (bind (_vallidpos1 _collidpos1 _size) (`/Game/Blueprints/CollisionsFunctions.DirectionTill_N_Hit` (`self.Box`) (`BlueprintMapLibrary.Map_Find` (`self.DirectionsVectors`) _array_element) (* (`BlueprintMapLibrary.Map_Find` (`self.Bonuses`) "NewEnumerator0") 1) 1 true))
        (bind _result (`BlueprintSetLibrary.Set_Union` (`self.ToDamagePos`) _vallidpos1))
        (set `self.ToDamagePos` _result)
        (bind _result_2 (`BlueprintSetLibrary.Set_Union` (`self.ToBreakPos`) _collidpos1))
        (set `self.ToBreakPos` _result_2)
        ;[1 0 1] Particles
        (bind _returnvalue (`NiagaraFunctionLibrary.SpawnSystemAtLocation` "/Game/Particle/P_Explosion.P_Explosion" (`SceneComponent.K2_GetComponentLocation` (`self.Box`)) (`BlueprintMapLibrary.Map_Find` (`self.DirectionsRotators`) _array_element)))
        (`FXSystemComponent.SetIntParameter` _returnvalue "Size" _size))
      ;[0.9896 0.1519 0] Blow
      (bind _result_3 (`BlueprintSetLibrary.Set_Union` (`self.ToBreakPos`) (`self.ToDamagePos`)))
      (bind _result_4 (`BlueprintSetLibrary.Set_ToArray` _result_3))
      (for _array_element_2 _result_4
        (bind _outhits (`/Game/Blueprints/CollisionsFunctions.PositionTest` _array_element_2))
        (for _array_element_3 _outhits
          (bind (_bblockinghit _binitialoverlap _time _distance _location _impactpoint _normal _impactnormal _physmat _hitactor) (`GameplayStatics.BreakHitResult` _array_element_3))
          (if (`KismetSystemLibrary.DoesImplementInterface` _hitactor "/Game/Blueprints/Interfaces/I_GameInteractions.I_GameInteractions_C")
            (message `/Game/Blueprints/Interfaces/I_GameInteractions.Blowed` _hitactor (`self.Damages`) (`KismetMathLibrary.Normal` (- _array_element_2 (`SceneComponent.K2_GetComponentLocation` (`self.Box`)))))))))
    (:`then_1`
      (`self.K2_DestroyActor`))))

(fn `UserConstructionScript`
  (`parent.UserConstructionScript`))