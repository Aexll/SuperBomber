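; Classic bomb actor, a child bomb class that triggers on spawn and explodes in four directions, then destroys itself.
; Detonate runs an inherited collision test per direction, sized by a bonus, sending bonus-scaled damage through I_GameInteractions to box-traced actors and the first-trace hit, such as a crate.
; Each direction spawns an explosion particle system whose size and time dilation follow the blast's extent.
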(event `self.ReceiveBeginPlay`
  (`parent.ReceiveBeginPlay`)
  (`self.Trigger`))

(event `self.Detonate`
  (`parent.Detonate`)
  (`|ExecutionSequence`
    (:`then_0`
      (for _array_element (`|MakeArray` "NewEnumerator0" "NewEnumerator1" "NewEnumerator2" "NewEnumerator3" :!type "/Game/Blueprints/Enums/E_Direction Enum")
        (bind _value (`BlueprintMapLibrary.Map_Find` (`self.DirectionsVectors`) _array_element))
        (bind (_firsttrace _boxtrace _extendsize) (`self.CollisionTest` _value (`BlueprintMapLibrary.Map_Find` (`self.Bonuses`) "NewEnumerator0")))
        (for _array_element_2 _boxtrace
          (bind (_bblockinghit _binitialoverlap _time _distance _location _impactpoint _normal _impactnormal _physmat _hitactor) (`GameplayStatics.BreakHitResult` _array_element_2))
          ;[1 0.03989 0] For each touched actors, blow them
          (if (`KismetSystemLibrary.DoesImplementInterface` _hitactor "/Game/Blueprints/Interfaces/I_GameInteractions.I_GameInteractions_C")
            (message `/Game/Blueprints/Interfaces/I_GameInteractions.Blowed` _hitactor (`self.GetDamagesWithBonus`) _value)))
        ;[1 0 1] Particles
        (bind _returnvalue (`NiagaraFunctionLibrary.SpawnSystemAtLocation` "/Game/Particle/P_Explosion.P_Explosion" (`SceneComponent.K2_GetComponentLocation` (`self.Box`)) (`BlueprintMapLibrary.Map_Find` (`self.DirectionsRotators`) _array_element)))
        (`NiagaraComponent.SetCustomTimeDilation` _returnvalue (* (/ 1.0 (`KismetMathLibrary.Conv_IntToDouble` (+ _extendsize 1))) 2.0))
        (`FXSystemComponent.SetIntParameter` _returnvalue "Size" _extendsize)
        (bind (_bblockinghit_2 _binitialoverlap_2 _time_2 _distance_2 _location_2 _impactpoint_2 _normal_2 _impactnormal_2 _physmat_2 _hitactor_2) (`GameplayStatics.BreakHitResult` _firsttrace))
        ;[0.3149 0 1] Crate interaction
        (if (`KismetSystemLibrary.DoesImplementInterface` _hitactor_2 "/Game/Blueprints/Interfaces/I_GameInteractions.I_GameInteractions_C")
          (message `/Game/Blueprints/Interfaces/I_GameInteractions.Blowed` _hitactor_2 (`self.GetDamagesWithBonus`) (* _normal_2 -1)))))
    (:`then_1`
      (`self.K2_DestroyActor`))))

(fn `GetDamagesWithBonus`
  (returns (Damages :type Integer))
  (return (* (+ (`BlueprintMapLibrary.Map_Find` (`self.Bonuses`) "NewEnumerator1") 1) (`self.Damages`))))

(fn `UserConstructionScript`
  (`parent.UserConstructionScript`))