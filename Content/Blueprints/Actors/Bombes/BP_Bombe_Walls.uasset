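; Bomb variant that builds walls of crates instead of exploding, arming itself on BeginPlay.
; On detonation it gathers valid positions in four directions, with reach set by a bonus, then spawns animated ToSpawn actors with bonus-scaled health.
; Positions failing the placement trace only show break particles tinted with the ToSpawn class's default color.
; It cannot be pushed, and being blown destroys it with directional break particles without detonating.
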(event `self.ReceiveBeginPlay`
  (`parent.ReceiveBeginPlay`)
  (`self.Trigger`))

(event `self.Detonate`
  (`parent.Detonate`)
  (`|ExecutionSequence`
    (:`then_0`
      ;[1 0.3901 0] GetLocations
      (for _array_element (`|MakeArray` "NewEnumerator0" "NewEnumerator1" "NewEnumerator2" "NewEnumerator3" :!type "/Game/Blueprints/Enums/E_Direction Enum")
        (bind _vallidpos1 (`/Game/Blueprints/CollisionsFunctions.DirectionTillHit` (`self.Box`) (`BlueprintMapLibrary.Map_Find` (`self.DirectionsVectors`) _array_element) (- (`BlueprintMapLibrary.Map_Find` (`self.Bonuses`) "NewEnumerator0") 1)))
        (bind _result (`BlueprintSetLibrary.Set_Union` (`self.ToCratePos`) _vallidpos1))
        (set `self.ToCratePos` _result))
      ;[0 0.3667 1] Spawn crates
      (bind _result_2 (`BlueprintSetLibrary.Set_ToArray` (`self.ToCratePos`)))
      (for _array_element_2 _result_2
        (bind (_outhits _returnvalue) (`/Game/Blueprints/CollisionsFunctions.PositionTest` _array_element_2))
        (if _returnvalue
          (bind _returnvalue_2 (`NiagaraFunctionLibrary.SpawnSystemAtLocation` "/Game/Particle/P_CreateBreak.P_CreateBreak" _array_element_2))
          (`FXSystemComponent.SetColorParameter` _returnvalue_2 "Color" (`.Color` (defaults `Object` (`self.ToSpawn`))))
          (`FXSystemComponent.SetVectorParameter` _returnvalue_2 "BlowDirection" (0.0 0.0 1.0))
          (else
            (bind _returnvalue_3 (`|SpawnActorFromClass` (`self.ToSpawn`) (`KismetMathLibrary.MakeTransform` _array_element_2) "Undefined" "OverrideRootScale" null false null))
            (`/Game/Blueprints/Actors/BP_Crate.SpawnAnimate` _returnvalue_3)
            (set `/Game/Blueprints/Actors/BP_Crate.Health` (+ (`BlueprintMapLibrary.Map_Find` (`self.Bonuses`) "NewEnumerator1") 1) _returnvalue_3)))))
    (:`then_1`
      (`self.K2_DestroyActor`))))

(event `/Game/Blueprints/Interfaces/I_GameInteractions.Blowed`
  (params (Damages :type Integer) (Direction :type "Vector Structure"))
  (bind _returnvalue (`NiagaraFunctionLibrary.SpawnSystemAtLocation` "/Game/Particle/P_CreateBreak.P_CreateBreak" (`SceneComponent.K2_GetComponentLocation` (`self.Box`))))
  (`FXSystemComponent.SetColorParameter` _returnvalue "Color" (`.Color` (defaults `Object` (`self.ToSpawn`))))
  (`FXSystemComponent.SetVectorParameter` _returnvalue "BlowDirection" Direction)
  (`self.K2_DestroyActor`))

(fn `Pushable`
  (params (Direction :type "/Game/Blueprints/Enums/E_Direction Enum" :default "NewEnumerator0"))
  (returns (Pushable :type Boolean))
  (return false))

(fn `UserConstructionScript`
  (`parent.UserConstructionScript`))