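; BP_Crate_Prefab is a crate actor that inherits its setup and game-start behavior from its parent class.
; Its own logic is on Tick, where a one-second Delay gates a Blowed call with minimal damage and an upward direction, so it fires repeatedly about once per second.
; BeginPlay, GameStart and the construction script only call their parent versions, and the overlap event is disabled.
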(event `self.ReceiveBeginPlay`
  (`parent.ReceiveBeginPlay`))

(event `self.ReceiveTick`
  (params (DeltaSeconds :type "Float (single-precision)"))
  (`parent.ReceiveTick` DeltaSeconds)
  (`KismetSystemLibrary.Delay` 1.0)
  (`/Game/Blueprints/Interfaces/I_GameInteractions.Blowed` 1 (0.0 0.0 1.0)))

(event `/Game/Blueprints/Interfaces/I_GameState.GameStart`
  (`parent.GameStart`))

(fn `UserConstructionScript`
  (`parent.UserConstructionScript`))