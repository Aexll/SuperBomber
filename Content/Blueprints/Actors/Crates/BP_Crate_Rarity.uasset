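; Breakable crate child Blueprint that rolls a random rarity at BeginPlay and drops bonus pickups when broken.
; Rarity climbs from its minimum on repeated low-odds rolls, is capped, and picks the crate color from the GameInstance.
; A randomized item count scaled by rarity fills a map of bonus types to quantities, which Break spawns as BP_Bonus actors.
; GameStart revives the crate without rerolling rarity or loot.
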(event `self.ReceiveBeginPlay`
  (bind _rarity_b (`self.Rarity_B`))
  (bind _content_b (`self.Content_B`))
  (bind _toadd_b (`self.ToAdd_B`))
  (set `self.Rarity_B` (`self.MinRarity_B`))
  (while (> (`KismetMathLibrary.RandomFloat`) 0.9)
    (`/Engine/EditorBlueprintResources/StandardMacros.IncrementInt` _rarity_b))
  (set `self.Rarity_B` (`KismetMathLibrary.Clamp` _rarity_b 0 (`self.MaxRarity_B`)))
  ;[0 0.008504 1] Set color
  (bind _asgi (cast `/Game/Blueprints/GI` (`GameplayStatics.GetGameInstance`))
    (:`then`
      (bind (_h _s _v) (`KismetMathLibrary.RGBToHSV` (`KismetMathLibrary.Conv_ColorToLinearColor` (`|GetArrayItem` (`/Game/Blueprints/GI.RarityColor` _asgi) (`self.Rarity_B`)))))
      (set `self.Color` (`KismetMathLibrary.HSVToRGB` _h _s _v)))
    (:`CastFailed`
      _))
  ;[1 0.4645 0] Set LootingTable
  (`BlueprintMapLibrary.Map_Clear` (`self.Content_B`))
  (for _ (range (`KismetMathLibrary.FTrunc` (* (`KismetMathLibrary.Conv_IntToDouble` (+ (`self.Rarity_B`) 1)) (`KismetMathLibrary.RandomFloatInRange` 0.0 2.0))))
    (bind _output_get (set `self.ToAdd_B` (`KismetArrayLibrary.Array_Random` (`|MakeArray` "NewEnumerator0" "NewEnumerator1" "NewEnumerator3" "NewEnumerator2" :!type "/Game/Blueprints/Enums/E_Bonus Enum"))))
    (bind (_value _returnvalue) (`BlueprintMapLibrary.Map_Find` (`self.Content_B`) _output_get))
    (if _returnvalue
      (`BlueprintMapLibrary.Map_Add` _content_b _toadd_b (+ _value 1))
      (else
        (`BlueprintMapLibrary.Map_Add` _content_b _toadd_b 1))))
  (`parent.ReceiveBeginPlay`))

(event `self.Break`
  (params (BlowDirection :type "Vector Structure"))
  (bind _content_b (`self.Content_B`))
  (`parent.Break` BlowDirection)
  ;[0.1875 1 0] Spawn Bonus
  (bind _keys (`BlueprintMapLibrary.Map_Keys` _content_b))
  (for _array_element _keys
    (for _ (range (`BlueprintMapLibrary.Map_Find` _content_b _array_element))
      (`|SpawnActorFromClass` "/Game/Blueprints/Actors/BP_Bonus.BP_Bonus_C" (`KismetMathLibrary.MakeTransform` (`SceneComponent.K2_GetComponentLocation` (`self.Box`))) "Undefined" "OverrideRootScale" null _array_element false null))))

(event `/Game/Blueprints/Interfaces/I_GameState.GameStart`
  (`self.Revive`))

(fn `UserConstructionScript`
  (`parent.UserConstructionScript`))