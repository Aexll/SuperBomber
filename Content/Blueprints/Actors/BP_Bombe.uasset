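; Grid-based bomb actor that detonates on a fuse timer or early when blown, and tracks its owning player's bomb count.
; BPMovement handles pushes, while freezing pauses the fuse, forces sliding and attaches a particle until a retriggerable delay expires.
; Detonate here only deactivates the bomb and clears freeze effects.
; Trace helpers, uncalled here, compute grid-snapped blast reach, valid cells along a direction and whether a push is unobstructed.
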(event `self.ReceiveBeginPlay`
  (`SceneComponent.K2_SetRelativeRotation` (`self.Scene`) (`KismetMathLibrary.MakeRotator` 0.0 0.0 (`KismetMathLibrary.RandomFloatInRange` 0.0 360.0)) false false)
  (set `self.DirectionsRotators` (`|MakeMap` "NewEnumerator0" (struct :`Yaw` 90.0) "NewEnumerator1" (struct :`Yaw` -90.0) "NewEnumerator2" (struct :`Yaw` 180.0) "NewEnumerator3" :!type "/Game/Blueprints/Enums/E_Direction Enum" :!valuetype "Rotator Structure"))
  (set `self.DirectionsVectors` (`|MakeMap` "NewEnumerator0" (0.0 1.0 0.0) "NewEnumerator1" (0.0 -1.0 0.0) "NewEnumerator2" (-1.0 0.0 0.0) "NewEnumerator3" (1.0 0.0 0.0) :!type "/Game/Blueprints/Enums/E_Direction Enum" :!valuetype "Vector Structure"))
  ;[0 0 1] Add bombe to count
  (bind _owningplayer (`self.OwningPlayer`)
    (:`then`
      (`/Engine/EditorBlueprintResources/StandardMacros.IncrementInt` (`/Game/Blueprints/Actors/BP_PlayerActor.BombeCount` _owningplayer)
        (:`  `
          _)))
    (:`else`
      _))
  (`FXSystemComponent.SetColorParameter` (`self.Niagara`) "Color" (`KismetMathLibrary.Conv_ColorToLinearColor` (`self.FireColor`))))

(event `self.ReceiveTick`
  (params (DeltaSeconds :type "Float (single-precision)")))

(event `Trigger`
  (bind _returnvalue (`KismetSystemLibrary.K2_SetTimerDelegate` (delegate `TryToDetonate`) (`self.FuseTime`)))
  (set `self.FuseTimer` _returnvalue))

(event `TryToDetonate`
  (if (`self.Active`)
    (`self.Detonate`)))

(event `Detonate`
  (set `self.Active` false)
  (bind _freezeparticle (`self.FreezeParticle`)
    (:`then`
      (`ActorComponent.K2_DestroyComponent` _freezeparticle))
    (:`else`)))

(event `self.ReceiveDestroyed`
  (bind _owningplayer (`self.OwningPlayer`)
    (:`then`
      (`/Engine/EditorBlueprintResources/StandardMacros.DecrementInt` (`/Game/Blueprints/Actors/BP_PlayerActor.BombeCount` _owningplayer)))
    (:`else`)))

(event `/Game/Blueprints/Interfaces/I_GameInteractions.Blowed`
  (params (Damages :type Integer) (Direction :type "Vector Structure"))
  (`KismetSystemLibrary.K2_PauseTimerHandle` (`self.FuseTimer`))
  (`self.TryToDetonate`))

(event `/Game/Blueprints/Interfaces/I_GameInteractions.Pushed`
  (params (Direction :type "/Game/Blueprints/Enums/E_Direction Enum" :default "NewEnumerator0") (Speed :type "Float (double-precision)"))
  (`/Game/Blueprints/BP_Movement.MoveTo` (`self.BP_Movement`) Direction Speed))

(event `/Game/Blueprints/Interfaces/I_GameInteractions.Freezed`
  (params (Level :type Integer))
  (bind _bp_movement (`self.BP_Movement`))
  (if (not (`self.IsFrozen`))
    (set `self.WasSliding` (`/Game/Blueprints/BP_Movement.Sliding` _bp_movement))
    (set `/Game/Blueprints/BP_Movement.Sliding` true _bp_movement)
    (set `self.IsFrozen` true)
    (`KismetSystemLibrary.K2_PauseTimerHandle` (`self.FuseTimer`))
    (bind _returnvalue (`NiagaraFunctionLibrary.SpawnSystemAttached` "/Game/Particle/P_Freezed.P_Freezed" (`self.Sphere`) "None" (0.0 0.0 0.0) (struct) "SnapToTarget"))
    (set `self.FreezeParticle` _returnvalue))
  (`KismetSystemLibrary.RetriggerableDelay` (`KismetMathLibrary.Conv_IntToDouble` Level))
  (`KismetSystemLibrary.K2_UnPauseTimerHandle` (`self.FuseTimer`))
  (set `self.IsFrozen` false)
  (set `/Game/Blueprints/BP_Movement.Sliding` (`self.WasSliding`) (`self.BP_Movement`))
  (bind _freezeparticle (`self.FreezeParticle`)
    (:`then`
      (`ActorComponent.K2_DestroyComponent` _freezeparticle))
    (:`else`)))

(fn `CollisionAtPosition`
  (params (Location :type "Vector Structure"))
  (returns (OutHits :type "Array of HitResult Structure") (ReturnValue :type Boolean))
  (bind (_outhits _returnvalue) (`KismetSystemLibrary.BoxTraceMulti` :`Start` Location :`End` Location :`HalfSize` (10.0 10.0 10.0) :`TraceChannel` "TraceTypeQuery3" :`DrawDebugType` "ForDuration"))
  (return _outhits _returnvalue))

(fn `CollisionsDirection`
  (params (NB :type Integer) (Direction :type "Vector Structure"))
  (returns (VallidPos1 :type "Array of Vector Structure") (CollidPos1 :type "Array of Vector Structure"))
  (locals (VallidPos :type "Array of Vector Structure") (CollidPos :type "Array of Vector Structure"))
  (for _index (range (+ NB 1))
    (bind _returnvalue (+ (* (`KismetMathLibrary.Normal` Direction) 100 _index) (`SceneComponent.K2_GetComponentLocation` (`self.Box`))))
    (bind (_outhits _returnvalue_2) (`/Game/Blueprints/CollisionsFunctions.PositionTest` _returnvalue))
    (`KismetArrayLibrary.Array_AddUnique` (select `bool` _returnvalue_2 :`false` (`local.VallidPos`) :`true` (`local.CollidPos`)) _returnvalue)
    (if _returnvalue_2
      (break)))
  (return (`local.VallidPos`) (`local.CollidPos`)))

(fn `CollisionTest`
  (params (Direction :type "Vector Structure") (Size :type Integer))
  (returns (FirstTrace :type "HitResult Structure") (BoxTrace :type "Array of HitResult Structure") (ExtendSize :type Integer))
  (locals (TressholdDisplacement :type Integer :default 50) (Locations :type "Array of Vector Structure"))
  (bind _returnvalue (`SceneComponent.K2_GetComponentLocation` (`self.Box`)))
  (bind _outhit (`KismetSystemLibrary.LineTraceSingle` _returnvalue (+ _returnvalue (* (`KismetMathLibrary.Normal` Direction) 100 Size)) "TraceTypeQuery3" false (`|MakeArray` self :!type "Actor Object Reference")))
  (bind (_bblockinghit _binitialoverlap _time _distance _location _impactpoint _normal _impactnormal _physmat _hitactor _hitcomponent _hitbonename _bonename _hititem _elementindex _faceindex _tracestart _traceend) (`GameplayStatics.BreakHitResult` _outhit))
  (bind _returnvalue_2 (+ _location (* _normal (`local.TressholdDisplacement`))))
  (bind _outhits (`KismetSystemLibrary.BoxTraceMulti` _tracestart (select `bool` _bblockinghit :`false` _traceend :`true` (`KismetMathLibrary.MakeVector` (.x (`KismetMathLibrary.Vector_SnappedToGrid` _returnvalue_2 100.0)) (.y (`KismetMathLibrary.Vector_SnappedToGrid` _returnvalue_2 100.0)) (.z _returnvalue_2))) (10.0 10.0 10.0) (struct) "TraceTypeQuery3"))
  (bind (_bblockinghit_2 _binitialoverlap_2 _time_2 _distance_2) (`GameplayStatics.BreakHitResult` _outhit))
  (return _outhit _outhits (select `bool` _bblockinghit_2 :`false` (`local.Size`) :`true` (/ _distance_2 100))))

(fn `Pushable`
  (params (Direction :type "/Game/Blueprints/Enums/E_Direction Enum" :default "NewEnumerator0"))
  (returns (Pushable :type Boolean))
  (bind _returnvalue (+ (`SceneComponent.K2_GetComponentLocation` (`self.Box`)) (* (`BlueprintMapLibrary.Map_Find` (`self.DirectionsVectors`) Direction) (.x (`BoxComponent.GetUnscaledBoxExtent` (`self.Box`))) 2.0)))
  (bind (_outhit _returnvalue_2) (`KismetSystemLibrary.BoxTraceSingle` _returnvalue _returnvalue (45.0 45.0 45.0) (struct) "TraceTypeQuery1" false (`|MakeArray` self :!type "Actor Object Reference") (select `bool` false :`true` "ForOneFrame" :!type "EDrawDebugTrace Enum") true (struct :`R` 1.0 :`A` 1.0) (struct :`G` 1.0 :`A` 1.0) 0.1))
  (return (not _returnvalue_2)))

(fn `ShowPosition`
  (params (Location :type "Vector Structure"))
  (`KismetSystemLibrary.BoxTraceMulti` :`Start` Location :`End` Location :`HalfSize` (10.0 10.0 10.0) :`TraceChannel` "TraceTypeQuery3" :`DrawDebugType` "ForDuration"))

(fn `UserConstructionScript`)