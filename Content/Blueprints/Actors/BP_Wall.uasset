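; BP_Wall is a wall actor with a Cube mesh that randomizes its color at construction.
; The construction script creates a dynamic instance of MI_Walls and offsets the Color parameter's hue by a random amount snapped to fixed steps, keeping saturation and value.
; Disconnected EventGraph logic, which never runs, would add the wall's transform to a BP_WallInstancer's instanced static mesh and destroy the actor.
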(event `self.ReceiveBeginPlay`)

(fn `UserConstructionScript`
  (bind _returnvalue (`PrimitiveComponent.CreateDynamicMaterialInstance` (`self.Cube`) 0 "/Game/Materials/MaterialsInstance/MI_Walls.MI_Walls" "None"))
  (bind _returnvalue_2 (`MaterialInstanceDynamic.K2_GetVectorParameterValue` _returnvalue "Color"))
  (bind (_h _s _v _a) (`KismetMathLibrary.RGBToHSV` _returnvalue_2))
  (`MaterialInstanceDynamic.SetVectorParameterValue` _returnvalue "Color" (`KismetMathLibrary.HSVToRGB` (+ _h (`KismetMathLibrary.GridSnap_Float` (`KismetMathLibrary.RandomFloatInRange` -200.0 200.0) 100.0)) _s _v _a)))