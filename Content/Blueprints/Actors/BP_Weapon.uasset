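; Bonus pickup actor that grants its BonusType (Power, Damages, Counts or Speed) to BP_PlayerActor on overlap, then spawns a type-colored Niagara burst and destroys itself.
; On spawn it tints its cylinder by type and drifts toward a random nearby horizontal offset through a Tick-driven gate, closed after one second.
; It spins continuously, reports itself as not pushable, and is destroyed when blown up or on GameStart.
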(event `self.ReceiveBeginPlay`
  (bind _returnvalue (`PrimitiveComponent.CreateDynamicMaterialInstance` (`self.Cylinder`) 0 "/Game/Materials/M_Bright.M_Bright" "None"))
  (`SceneComponent.K2_SetRelativeRotation` (`self.Scene`) (`KismetMathLibrary.MakeRotator` 0.0 0.0 (`KismetMathLibrary.RandomFloatInRange` 0.0 360.0)) false false)
  (`MaterialInstanceDynamic.SetVectorParameterValue` _returnvalue "Color" (select `/Game/Blueprints/Enums/E_Bonus` (`self.BonusType`) :`NewEnumerator0` (struct :`R` 1.0 :`G` 0.298155 :`A` 1.0) :`NewEnumerator1` (struct :`R` 1.0 :`A` 1.0) :`NewEnumerator3` (struct :`G` 0.044348 :`B` 1.0 :`A` 1.0) :`NewEnumerator2` (struct :`R` 0.135347 :`G` 1.0 :`A` 1.0) :!type "LinearColor Structure"))
  (`KismetSystemLibrary.K2_SetTimerDelegate` (delegate `StopMoving`) 1.0)
  (set `self.Target` (`KismetMathLibrary.MakeVector` (.x (* (`KismetMathLibrary.RandomUnitVector`) 75)) (.y (* (`KismetMathLibrary.RandomUnitVector`) 75))))
  (goto _label :!via `Open`))

(event `self.ReceiveTick`
  (params (DeltaSeconds :type "Float (single-precision)"))
  (`SceneComponent.K2_AddRelativeRotation` (`self.Scene`) (struct :`Yaw` 1.0) false false)
  (`/Engine/EditorBlueprintResources/StandardMacros.Gate` true :!label _label
    (:`Exit`
      (bind _output_get (set `self.Current` (`KismetMathLibrary.VInterpTo` (`self.Current`) (`self.Target`) 0.01 1.0)))
      (`SceneComponent.K2_SetRelativeLocation` (`self.Scene`) _output_get false false))))

(event `StopMoving`
  (goto _label :!via `Close`))

(event `self.Box.OnComponentBeginOverlap`
  (params (OverlappedComponent :type "PrimitiveComponent Object Reference") (OtherActor :type "Actor Object Reference") (OtherComp :type "PrimitiveComponent Object Reference") (OtherBodyIndex :type Integer) (bFromSweep :type Boolean) (SweepResult :type "HitResult Structure (by ref)"))
  (bind _asbp_player_actor (cast `/Game/Blueprints/Actors/BP_PlayerActor` OtherActor))
  (`/Game/Blueprints/Actors/BP_PlayerActor.GetBonus` _asbp_player_actor (`self.BonusType`) 1)
  (bind _returnvalue (`NiagaraFunctionLibrary.SpawnSystemAtLocation` "/Game/Particle/P_BonusCollect.P_BonusCollect" (`SceneComponent.K2_GetComponentLocation` (`self.Cylinder`)) (`KismetMathLibrary.ComposeRotators` (`SceneComponent.RelativeRotation` (`self.Scene`)) (struct :`Yaw` 90.0))))
  (`NiagaraComponent.SetVariableLinearColor` _returnvalue "Color" (select `/Game/Blueprints/Enums/E_Bonus` (`self.BonusType`) :`NewEnumerator0` (struct :`R` 1.0 :`G` 0.298155 :`A` 1.0) :`NewEnumerator1` (struct :`R` 1.0 :`A` 1.0) :`NewEnumerator3` (struct :`G` 0.044348 :`B` 1.0 :`A` 1.0) :`NewEnumerator2` (struct :`R` 0.135347 :`G` 1.0 :`A` 1.0) :!type "LinearColor Structure"))
  (`self.K2_DestroyActor`))

(event `Collect`)

(event `/Game/Blueprints/Interfaces/I_GameInteractions.Blowed`
  (params (Damages :type Integer) (Direction :type "Vector Structure"))
  (`self.K2_DestroyActor`))

(event `/Game/Blueprints/Interfaces/I_GameState.GameStart`
  (`self.K2_DestroyActor`))

(fn `Pushable`
  (params (Direction :type "/Game/Blueprints/Enums/E_Direction Enum" :default "NewEnumerator0"))
  (returns (Pushable :type Boolean))
  (return false))

(fn `UserConstructionScript`)