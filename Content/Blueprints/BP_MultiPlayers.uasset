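; Local multiplayer manager actor that spawns one BP_PlayerActor per game-instance player count at editable spawn points, previewed as instanced meshes in the construction script.
; It forwards every key press and release to all players; W also sends a freeze message to game-interaction actors.
; Each tick, a shared camera eases toward the players' bounds, clamped to the play area, and zooms with their spread.
; When one or fewer players remain alive, it notifies the game mode.
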(event `self.ReceiveBeginPlay`
  (bind _asgi (cast `/Game/Blueprints/GI` (`GameplayStatics.GetGameInstance`)))
  (set `self.GI` _asgi)
  ;[0 0 1] Creating Players
  (for _index (range (`/Game/Blueprints/GI.PlayersNB` (`self.GI`)))
    (bind _returnvalue (`|SpawnActorFromClass` "/Game/Blueprints/Actors/BP_PlayerActor.BP_PlayerActor_C" (`KismetMathLibrary.MakeTransform` (`self.K2_GetActorLocation`)) "Undefined" "OverrideRootScale" null _index null))
    (`KismetArrayLibrary.Array_Add` (`self.PlayersActors`) _returnvalue))
  (`self.SpawnPlayers`))

(event `self.ReceiveTick`
  (params (DeltaSeconds :type "Float (single-precision)"))
  ;[1 0 1] Set cam location
  (`self.SetCameraLocation`))

(event `Key|AnyKey`
  (params (Key :type "Key Structure"))
  ;[1 0.1355 0] Input System
  (:`Pressed`
    (for _array_element (`self.PlayersActors`)
      (`/Game/Blueprints/Actors/BP_PlayerActor.Input_Pressed` _array_element Key)))
  (:`Released`
    (for _array_element_2 (`self.PlayersActors`)
      (`/Game/Blueprints/Actors/BP_PlayerActor.Input_Release` _array_element_2 Key))))

(event `SpawnPlayers`
  (bind _spawnpoints (`self.SpawnPoints`))
  ;[0 1 0] Start Game
  (for (_array_element _array_index) (`self.PlayersActors`)
    (`self.K2_SetActorLocation` _array_element (+ (`self.K2_GetActorLocation`) (* (`KismetMathLibrary.SelectVector` (`|GetArrayItem` _spawnpoints _array_index) (0.0 0.0 0.0) (`KismetArrayLibrary.Array_IsValidIndex` _spawnpoints _array_index)) 100.0)) false false)))

(event `/Game/Blueprints/Interfaces/I_GameInteractions.PlayerDied`
  (params (Player :type "/Game/Blueprints/Actors/BP_PlayerActor Object Reference"))
  ;[1 0.3714 0] if only one player is alive, win the game
  (bind _aliveplayers (`self.GetAlivePlayers`))
  (if (<= (`KismetArrayLibrary.Array_Length` _aliveplayers) 1)
    (bind _asgm (cast `/Game/Blueprints/GM` (`GameplayStatics.GetGameMode`)))
    (`/Game/Blueprints/GM.GM_GameEnd` _asgm (`|GetArrayItem` _aliveplayers))))

(event `/Game/Blueprints/Interfaces/I_GameState.GameStart`
  ;[1 0.3141 0] On start, spawn players
  (`self.SpawnPlayers`))

(event `Key|W`
  (params (Key :type "Key Structure"))
  (:`Pressed`
    (`KismetSystemLibrary.PrintString` "Proute")
    (bind _outactors (`GameplayStatics.GetAllActorsWithInterface` "/Game/Blueprints/Interfaces/I_GameInteractions.I_GameInteractions_C"))
    (for _array_element _outactors
      (message `/Game/Blueprints/Interfaces/I_GameInteractions.Freezed` _array_element 1))))

(fn `GetAlivePlayers`
  (returns (AlivePlayers :type "Array of /Game/Blueprints/Actors/BP_PlayerActor Object Reference"))
  (locals (TempAlivePlayers :type "Array of /Game/Blueprints/Actors/BP_PlayerActor Object Reference"))
  (for _array_element (`self.PlayersActors`)
    (if (`/Game/Blueprints/Actors/BP_PlayerActor.Alive` _array_element)
      (`KismetArrayLibrary.Array_Add` (`local.TempAlivePlayers`) _array_element)))
  (return (`local.TempAlivePlayers`)))

(fn `Pushable`
  (params (Direction :type "/Game/Blueprints/Enums/E_Direction Enum" :default "NewEnumerator0"))
  (returns (Pushable :type Boolean))
  (return false))

(fn `SetCameraLocation`
  (locals (Farest :type "Vector Structure"))
  (bind _playareasize (`self.PlayAreaSize`))
  (bind _returnvalue (`SceneComponent.K2_GetComponentLocation` (`self.Box`)))
  (bind _returnvalue_2 (* (100.0 100.0 0.0) (`self.CameraInerMapBoundMargin`)))
  ;[0 0 1] CameraPos
  (bind (_center _boxextent) (`GameplayStatics.GetActorArrayBounds` (`self.PlayersActors`)))
  (bind _returnvalue_3 (* (`self.CameraOffset`) 100 (/ (.y _boxextent) 200.0)))
  (set `self.DestinationCamPos` (`KismetMathLibrary.Vector_BoundedToBox` _center (+ _returnvalue (+ (/ (* _playareasize -100) 2) _returnvalue_2) _returnvalue_3) (+ _returnvalue (- (/ (* _playareasize 100) 2) _returnvalue_2) _returnvalue_3)))
  (bind _output_get (set `self.CurrentCamPos` (`KismetMathLibrary.VInterpTo` (`self.CurrentCamPos`) (`self.DestinationCamPos`) (`self.CamSpeed`) 1.0)))
  (`SceneComponent.K2_SetWorldLocation` (`self.CameraPivot`) _output_get false false)
  ;[1 0.3282 0] Camera distance
  (bind _output_get_2 (set `self.DestinationDistance` (`KismetMathLibrary.FClamp` (+ (* (`KismetMathLibrary.VSize` _boxextent) 1.5) 100.0) 1000.0 100000.0)))
  (bind _returnvalue_4 (`KismetMathLibrary.FInterpTo` (`self.CurrentDistance`) _output_get_2 (`self.CamSpeed`) 1.0))
  (set `self.CurrentDistance` _returnvalue_4)
  (set `SpringArmComponent.TargetArmLength` _returnvalue_4 (`self.SpringArm`)))

(fn `ShowGride`
  (bind _z (.z (`SceneComponent.K2_GetComponentLocation` (`self.Box`))))
  (for _index (range -5 6)
    (for _index_2 (range -5 6)
      (bind _returnvalue (`KismetMathLibrary.MakeVector` (.x (`KismetMathLibrary.Vector_SnappedToGrid` (`KismetMathLibrary.MakeVector` (+ (* _index_2 100) (.x (`SceneComponent.K2_GetComponentLocation` (`self.Box`)))) (+ (* _index 100) (.y (`SceneComponent.K2_GetComponentLocation` (`self.Box`)))) _z) 100.0)) (.y (`KismetMathLibrary.Vector_SnappedToGrid` (`KismetMathLibrary.MakeVector` (+ (* _index_2 100) (.x (`SceneComponent.K2_GetComponentLocation` (`self.Box`)))) (+ (* _index 100) (.y (`SceneComponent.K2_GetComponentLocation` (`self.Box`)))) _z) 100.0)) (- _z 40.0)))
      (`KismetSystemLibrary.BoxTraceSingle` :`Start` _returnvalue :`End` _returnvalue :`HalfSize` (10.0 10.0 0.0) :`TraceChannel` "TraceTypeQuery1" :`DrawDebugType` "Persistent" :`TraceColor` (struct :`B` 1.0 :`A` 1.0) :`TraceHitColor` (struct :`R` 1.0 :`B` 1.0 :`A` 1.0)))))

(fn `UserConstructionScript`
  (bind _instancedstaticmesh (`self.InstancedStaticMesh`))
  (`SceneComponent.SetWorldScale3D` (`self.PlayArea`) (`self.PlayAreaSize`))
  (set `self.CurrentCamPos` (+ (`SceneComponent.K2_GetComponentLocation` (`self.CameraPivot`)) (0.0 0.0 100.0)))
  ;[1 0.3333 0] Spawnpoint preview
  (for (_array_element _array_index) (`self.SpawnPoints`)
    (if (`InstancedStaticMeshComponent.IsValidInstance` _instancedstaticmesh _array_index)
      (bind _returnvalue (* _array_element 100.0))
      (`InstancedStaticMeshComponent.UpdateInstanceTransform` _instancedstaticmesh _array_index (`KismetMathLibrary.MakeTransform` _returnvalue (struct :`Yaw` 90.0) (2.0 2.0 2.0)) false false false)
      (else
        (`InstancedStaticMeshComponent.AddInstance` _instancedstaticmesh (`KismetMathLibrary.MakeTransform` _returnvalue (struct :`Yaw` 90.0) (2.0 2.0 2.0)) false)))))