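; GM is a game manager Blueprint that moves a match between waiting, running and ended states, entering the waiting state on BeginPlay.
; Each transition sets State and broadcasts a message to every I_GameState actor, with the end message carrying the PlayerWin result.
; Starting resets and runs a looping one-second countdown that triggers game end at zero; ending pauses it.
; Separate start, end and wait events only print debug text.
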(event `self.ReceiveBeginPlay`
  (`self.GM_WaitToStart`))

(event `GM_GameEnd`
  (params (PlayerWin :type "/Game/Blueprints/Actors/BP_PlayerActor Object Reference"))
  ;[0 0.3698 0.01236] State
  (set `self.State` "NewEnumerator1")
  ;[0 0 1] Timer
  (`self.PauseTimer`)
  ;[1 0.4695 0.1302] Messages
  (bind _outactors (`GameplayStatics.GetAllActorsWithInterface` "/Game/Blueprints/Interfaces/I_GameState.I_GameState_C"))
  (for _array_element _outactors
    (message `/Game/Blueprints/Interfaces/I_GameState.GameEnd` _array_element PlayerWin)))

(event `GM_StartGame`
  ;[0 0.3698 0.01236] State
  (set `self.State` "NewEnumerator0")
  ;[0 0 1] Timer
  (`self.ResetTimer`)
  (`self.StartTimer`)
  ;[1 0.4695 0.1302] Messages
  (bind _outactors (`GameplayStatics.GetAllActorsWithInterface` "/Game/Blueprints/Interfaces/I_GameState.I_GameState_C"))
  (for _array_element _outactors
    (message `/Game/Blueprints/Interfaces/I_GameState.GameStart` _array_element)))

(event `GM_WaitToStart`
  ;[0 0.3698 0.01236] State
  (set `self.State` "NewEnumerator2")
  ;[1 0.4695 0.1302] Messages
  (bind _outactors (`GameplayStatics.GetAllActorsWithInterface` "/Game/Blueprints/Interfaces/I_GameState.I_GameState_C"))
  (for _array_element _outactors
    (message `/Game/Blueprints/Interfaces/I_GameState.GameWaitToStart` _array_element)))

(event `/Game/Blueprints/Interfaces/I_GameState.GameStart`
  (`KismetSystemLibrary.PrintString` "Game Start"))

(event `/Game/Blueprints/Interfaces/I_GameState.GameEnd`
  (params (PlayerWon :type "/Game/Blueprints/Actors/BP_PlayerActor Object Reference"))
  (`KismetSystemLibrary.PrintString` "Game End"))

(event `/Game/Blueprints/Interfaces/I_GameState.GameWaitToStart`
  (`KismetSystemLibrary.PrintString` "Ready to start"))

(event `ResetTimer`
  ;[0 0 1] Timer
  (set `self.TimerTime` (`self.DefaultTime`)))

(event `PauseTimer`
  ;[0 0 1] Timer
  (`KismetSystemLibrary.K2_PauseTimerHandle` (`self.Timer`)))

(event `StartTimer`
  ;[0 0 1] Timer
  (if (`KismetSystemLibrary.K2_IsValidTimerHandle` (`self.Timer`))
    (`KismetSystemLibrary.K2_UnPauseTimerHandle` (`self.Timer`))
    (else
      (bind _returnvalue (`KismetSystemLibrary.K2_SetTimerDelegate` (delegate `TimerTick`) 1.0 true))
      (set `self.Timer` _returnvalue))))

(event `TimerTick`
  ;[0 0 1] Timer
  (bind _result (`/Engine/EditorBlueprintResources/StandardMacros.DecrementInt` (`self.TimerTime`))
    (:`  `
      (if (<= _result 0)
        (`self.GM_GameEnd` null)))))

(fn `UserConstructionScript`)