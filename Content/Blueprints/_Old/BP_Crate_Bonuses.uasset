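; Breakable crate that holds random bonus pickups and is reused on each game start rather than destroyed.
; BeginPlay and Act roll a rarity from a minimum, tint the crate with the GameInstance's rarity color, and fill a type-to-count loot map scaled by rarity.
; Break plays a directional Niagara effect, hides the crate without collision, and spawns a BP_Bonus per loot entry count.
; GameStart rerolls and revives it; SpawnAnimate reveals it after a spawn effect.
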(event `self.ReceiveBeginPlay`
  (bind _rarity (`self.Rarity`))
  (bind _content (`self.Content`))
  (bind _toadd (`self.ToAdd`))
  (set `self.Rarity` (`self.MinumRarity`) :!label _label)
  (while (> (`KismetMathLibrary.RandomFloat`) 0.9)
    (`/Engine/EditorBlueprintResources/StandardMacros.IncrementInt` _rarity))
  (set `self.Rarity` (`KismetMathLibrary.Clamp` _rarity 0 6))
  ;[0 0.008504 1] Set color
  (bind _returnvalue (`PrimitiveComponent.CreateDynamicMaterialInstance` (`self.Cube`) 0 "/Game/Materials/MaterialsInstance/MI_Crate.MI_Crate" "None"))
  (bind _asgi (cast `/Game/Blueprints/GI` (`GameplayStatics.GetGameInstance`))
    (:`then`
      (bind (_h _s _v) (`KismetMathLibrary.RGBToHSV` (`KismetMathLibrary.Conv_ColorToLinearColor` (`|GetArrayItem` (`/Game/Blueprints/GI.RarityColor` _asgi) (`self.Rarity`)))))
      (`MaterialInstanceDynamic.SetVectorParameterValue` _returnvalue "Color" (`KismetMathLibrary.HSVToRGB` _h _s _v)))
    (:`CastFailed`
      _))
  ;[1 0.4645 0] Set LootingTable
  (`BlueprintMapLibrary.Map_Clear` (`self.Content`))
  (for _ (range (`KismetMathLibrary.FTrunc` (* (`KismetMathLibrary.Conv_IntToDouble` (+ (`self.Rarity`) 1)) (`KismetMathLibrary.RandomFloatInRange` 0.0 2.0))))
    (bind _output_get (set `self.ToAdd` (`KismetArrayLibrary.Array_Random` (`|MakeArray` "NewEnumerator0" "NewEnumerator1" "NewEnumerator3" "NewEnumerator2" :!type "/Game/Blueprints/Enums/E_Bonus Enum"))))
    (bind (_value _returnvalue_2) (`BlueprintMapLibrary.Map_Find` _content _output_get))
    (if _returnvalue_2
      (`BlueprintMapLibrary.Map_Add` _content _toadd (+ _value 1))
      (else
        (`BlueprintMapLibrary.Map_Add` _content _toadd 1)))))

(event `Act`
  (goto _label))

(event `Break`
  (params (BlowDirection :type "Vector Structure"))
  (bind _content (`self.Content`))
  (bind (_returnvalue_location _returnvalue_rotation _returnvalue_scale) (`KismetMathLibrary.BreakTransform` (`SceneComponent.K2_GetComponentToWorld` (`self.Box`))))
  (bind _returnvalue (`NiagaraFunctionLibrary.SpawnSystemAtLocation` "/Game/Particle/P_CreateBreak.P_CreateBreak" _returnvalue_location _returnvalue_rotation _returnvalue_scale))
  (`FXSystemComponent.SetVectorParameter` _returnvalue "BlowDirection" BlowDirection)
  (`KismetSystemLibrary.DelayUntilNextTick`)
  (`self.Kill`)
  ;[0.1875 1 0] Spawn Bonus
  (bind _keys (`BlueprintMapLibrary.Map_Keys` _content))
  (for _array_element _keys
    (for _ (range (`BlueprintMapLibrary.Map_Find` _content _array_element))
      (`|SpawnActorFromClass` "/Game/Blueprints/Actors/BP_Bonus.BP_Bonus_C" (`KismetMathLibrary.MakeTransform` (`SceneComponent.K2_GetComponentLocation` (`self.Box`))) "Undefined" "OverrideRootScale" null _array_element null))))

(event `/Game/Blueprints/Interfaces/I_GameState.GameStart`
  (`self.Act`)
  (`self.Revive`))

(event `Kill`
  (`SceneComponent.SetVisibility` (`self.Box`) false true)
  (`PrimitiveComponent.SetCollisionEnabled` (`self.Box`) "NoCollision"))

(event `Revive`
  (`SceneComponent.SetVisibility` (`self.Box`) true true)
  (`PrimitiveComponent.SetCollisionEnabled` (`self.Box`) "QueryAndPhysics"))

(event `Hide`
  (`SceneComponent.SetVisibility` (`self.Box`) false true))

(event `SpawnAnimate`
  (`self.Hide`)
  (`NiagaraFunctionLibrary.SpawnSystemAtLocation` "/Game/Particle/P_SpawnCrate.P_SpawnCrate" (`SceneComponent.K2_GetComponentLocation` (`self.Cube`)))
  (`KismetSystemLibrary.Delay` 0.5)
  (`self.Revive`))

(fn `UserConstructionScript`)