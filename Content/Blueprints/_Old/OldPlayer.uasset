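; Two-player input Blueprint that gathers movement input for P1 and P2; nothing in this file moves them.
; Each player's Up and Right axes scale the forward vectors of V and H components by PlayerSpeed, accumulating into per-index movement and direction arrays.
; PlayerPendingMovement returns both values and clears direction, while PlayerConsumeMovement returns and clears movement.
; The construction script hides player and axis components in game unless Debug is set.
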(event `self.ReceiveBeginPlay`
  (bind _array (`|MakeArray` (0.0 0.0 0.0) (0.0 0.0 0.0) :!type "Vector Structure"))
  (set `self.Players` (`|MakeArray` (`self.P1`) (`self.P2`)))
  (set `self.MovementInput` _array)
  (set `self.DirectionInput` _array))

(event `self.ReceiveTick`
  (params (DeltaSeconds :type "Float (single-precision)")))

(event `InputAxis|P1Up`
  (params (AxisValue :type "Float (single-precision)"))
  (`self.Player_AddMovementInput` 0 (* AxisValue (`SceneComponent.GetForwardVector` (`self.V1`))) (`self.PlayerSpeed`)))

(event `InputAxis|P1Right`
  (params (AxisValue :type "Float (single-precision)"))
  (`self.Player_AddMovementInput` 0 (* AxisValue (`SceneComponent.GetForwardVector` (`self.H1`))) (`self.PlayerSpeed`)))

(event `InputAxis|P2Up`
  (params (AxisValue :type "Float (single-precision)"))
  (`self.Player_AddMovementInput` 1 (* AxisValue (`SceneComponent.GetForwardVector` (`self.V2`))) (`self.PlayerSpeed`)))

(event `InputAxis|P2Right`
  (params (AxisValue :type "Float (single-precision)"))
  (`self.Player_AddMovementInput` 1 (* AxisValue (`SceneComponent.GetForwardVector` (`self.H2`))) (`self.PlayerSpeed`)))

(fn `Player_AddMovementInput`
  (params (Index :type Integer) (Input :type "Vector Structure") (Speed :type "Float (double-precision)"))
  (bind _returnvalue (* Input Speed))
  (`KismetArrayLibrary.Array_Set` (`self.MovementInput`) Index (+ (`|GetArrayItem` (`self.MovementInput`) Index) _returnvalue) true)
  (`KismetArrayLibrary.Array_Set` (`self.DirectionInput`) Index (+ _returnvalue (`|GetArrayItem` (`self.DirectionInput`) Index)) true))

(fn `Player_ConsumeMovement`
  (params (Index :type Integer))
  (returns (NewParam :type "Vector Structure"))
  (locals (Input :type "Vector Structure"))
  (bind _movementinput (`self.MovementInput`))
  (set `local.Input` (`|GetArrayItem` _movementinput Index))
  (`KismetArrayLibrary.Array_Set` _movementinput Index (0.0 0.0 0.0) true)
  (return (`local.Input`)))

(fn `Player_PendingMovement`
  (params (Index :type Integer))
  (returns (MovmentInput :type "Vector Structure") (DirectionInput :type "Vector Structure"))
  (locals (DrectionInput_1 :type "Vector Structure"))
  (bind _directioninput (`self.DirectionInput`))
  (set `local.DrectionInput_1` (`|GetArrayItem` _directioninput Index))
  (`KismetArrayLibrary.Array_Set` _directioninput Index)
  (return (`|GetArrayItem` (`self.MovementInput`) Index) (`local.DrectionInput_1`)))

(fn `UserConstructionScript`
  (`SceneComponent.SetHiddenInGame` (`self.P2`) (not (`self.Debug`)) false)
  (`SceneComponent.SetHiddenInGame` (`self.H2`) (not (`self.Debug`)) false)
  (`SceneComponent.SetHiddenInGame` (`self.V2`) (not (`self.Debug`)) false)
  (`SceneComponent.SetHiddenInGame` (`self.P1`) (not (`self.Debug`)) false)
  (`SceneComponent.SetHiddenInGame` (`self.H1`) (not (`self.Debug`)) false)
  (`SceneComponent.SetHiddenInGame` (`self.V1`) (not (`self.Debug`)) false))