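; Movement component for OldPlayer that gives two players grid-stepped movement with meshes that slide between cells.
; Each tick it clamps each player's pending input and offsets that player's mesh from its collision component.
; Crossing the block threshold consumes the input and steps the collider one cell unless a directional box trace is blocked.
; After a step, the mesh and input are re-seeded on the opposite side, keeping motion continuous.
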(event `self.ReceiveBeginPlay`
  (bind _asold_player (cast `/Game/Blueprints/_Old/OldPlayer` (`self.GetOwner`)))
  (bind _output_get (set `self.As Player` _asold_player))
  (set `self.P1` (`/Game/Blueprints/_Old/OldPlayer.P1` _output_get))
  (set `self.P2` (`/Game/Blueprints/_Old/OldPlayer.P2` _output_get))
  (set `self.P1_Mesh` (`/Game/Blueprints/_Old/OldPlayer.P1_Mesh` _output_get))
  (set `self.P2_Mesh` (`/Game/Blueprints/_Old/OldPlayer.P2_Mesh` _output_get)))

(event `self.ReceiveTick`
  (params (DeltaSeconds :type "Float (single-precision)"))
  (`self.MovePlayer` (`|MakeArray` (`self.P1`) (`self.P2`)) (`|MakeArray` (`self.P1_Mesh`) (`self.P2_Mesh`))))

(fn `AfterBoxMoved`)

(fn `CollisionDefine`
  (params (P :type "BoxComponent Object Reference"))
  (returns (Up1 :type Boolean) (Down1 :type Boolean) (Right1 :type Boolean) (Left1 :type Boolean))
  (locals (Up :type Boolean) (Down :type Boolean) (Right :type Boolean) (Left :type Boolean))
  (`|ExecutionSequence`
    (:`then_0`
      (bind (_outhit _returnvalue) (`self.TestCollide` "NewEnumerator0" (`local.P`)))
      (set `local.Up` _returnvalue))
    (:`then_1`
      (bind (_outhit_2 _returnvalue_2) (`self.TestCollide` "NewEnumerator1" (`local.P`)))
      (set `local.Down` _returnvalue_2))
    (:`then_2`
      (bind (_outhit_3 _returnvalue_3) (`self.TestCollide` "NewEnumerator2" (`local.P`)))
      (set `local.Right` _returnvalue_3))
    (:`then_3`
      (bind (_outhit_4 _returnvalue_4) (`self.TestCollide` "NewEnumerator3" (`local.P`)))
      (set `local.Left` _returnvalue_4))
    (:`then_4`
      (return (`local.Up`) (`local.Down`) (`local.Right`) (`local.Left`)))))

(fn `MovePlayer`
  (params (PlayersColid :type "Array of BoxComponent Object Reference") (PlayersMesh :type "Array of StaticMeshComponent Object Reference"))
  (locals (P_Index :type Integer) (P_Mesh :type "StaticMeshComponent Object Reference") (P :type "BoxComponent Object Reference") (PendingMovement :type "Vector Structure" :default (0.0 0.0 0.0)) (ConsumedMovement :type "Vector Structure") (UpCollide :type Boolean :default false) (DownCollide :type Boolean) (RightCollide :type Boolean) (LeftCollide :type Boolean))
  (bind _blocksize (`self.BlockSize`))
  (bind _pendingmovement (`local.PendingMovement`))
  (bind _x (.x (`local.PendingMovement`)))
  (bind _y (.y (`local.PendingMovement`)))
  (bind _returnvalue (* _blocksize -1.0))
  (bind _movementinput (`/Game/Blueprints/_Old/OldPlayer.MovementInput` (`self.As Player`)))
  (bind _returnvalue_2 (> (`KismetMathLibrary.VSize` _pendingmovement) (* (`self.BoundBox`) 1.1)))
  (for _index (range (+ (`KismetArrayLibrary.Array_LastIndex` PlayersColid) 1))
    (set `local.P_Index` _index)
    (set `local.P` (`|GetArrayItem` (`local.PlayersColid`) (`local.P_Index`)))
    (set `local.P_Mesh` (`|GetArrayItem` (`local.PlayersMesh`) (`local.P_Index`)))
    (bind (_movmentinput _directioninput) (`/Game/Blueprints/_Old/OldPlayer.Player_PendingMovement` (`self.As Player`) (`local.P_Index`)))
    (`KismetSystemLibrary.PrintString` (`KismetStringLibrary.Conv_VectorToString` _movmentinput))
    (set `local.PendingMovement` _movmentinput)
    (bind (_up1 _down1 _right1 _left1) (`self.CollisionDefine` (`local.P`)))
    (set `local.UpCollide` _up1)
    (set `local.DownCollide` _down1)
    (set `local.RightCollide` _right1)
    (set `local.LeftCollide` _left1)
    (if _returnvalue_2
      (`KismetArrayLibrary.Array_Set` _movementinput (`local.P_Index`) (+ (`|GetArrayItem` _movementinput) (* _directioninput -1.0)) true))
    (set `local.PendingMovement` (select `bool` _returnvalue_2 :`false` _pendingmovement :`true` (* (`KismetMathLibrary.Normal` _pendingmovement) (`self.BoundBox`))))
    (`SceneComponent.K2_SetRelativeLocation` (`local.P_Mesh`) (* (`local.PendingMovement`) 10) false false)
    ;[1 0.3333 0] Test if crossed the box
    (if (or (>= _x _blocksize) (<= _x _returnvalue) (>= _y _blocksize) (<= _y _returnvalue))
      (`/Game/Blueprints/_Old/OldPlayer.Player_ConsumeMovement` (`self.As Player`) (`local.P_Index`))
      (set `local.ConsumedMovement` (`local.PendingMovement`))
      (`|ExecutionSequence`
        (:`then_0`
          (if (and (not (`local.UpCollide`)) (>= (.y (`local.ConsumedMovement`)) (`self.BlockSize`)))
            (`SceneComponent.K2_AddWorldOffset` (`local.P`) (* (`KismetMathLibrary.MakeVector` 0.0 10.0) 10) false false)
            (`SceneComponent.K2_SetRelativeLocation` (`local.P_Mesh`) (0.0 -50.0 0.0) false false)
            (`/Game/Blueprints/_Old/OldPlayer.Player_AddMovementInput` (`self.As Player`) (`local.P_Index`) (0.0 -4.9 0.0) 1.0)))
        (:`then_1`
          (if (and (not (`local.DownCollide`)) (<= (.y (`local.ConsumedMovement`)) (* (`self.BlockSize`) -1.0)))
            (`SceneComponent.K2_AddWorldOffset` (`local.P`) (* (`KismetMathLibrary.MakeVector` 0.0 -10.0) 10) false false)
            (`SceneComponent.K2_SetRelativeLocation` (`local.P_Mesh`) (0.0 50.0 0.0) false false)
            (`/Game/Blueprints/_Old/OldPlayer.Player_AddMovementInput` (`self.As Player`) (`local.P_Index`) (0.0 4.9 0.0) 1.0)))
        (:`then_2`
          (if (and (not (`local.RightCollide`)) (>= (.x (`local.ConsumedMovement`)) (`self.BlockSize`)))
            (`SceneComponent.K2_AddWorldOffset` (`local.P`) (* (`KismetMathLibrary.MakeVector` 10.0) 10) false false)
            (`SceneComponent.K2_SetRelativeLocation` (`local.P_Mesh`) (-50.0 0.0 0.0) false false)
            (`/Game/Blueprints/_Old/OldPlayer.Player_AddMovementInput` (`self.As Player`) (`local.P_Index`) (-4.9 0.0 0.0) 1.0)))
        (:`then_3`
          (if (and (not (`local.LeftCollide`)) (<= (.x (`local.ConsumedMovement`)) (* (`self.BlockSize`) -1.0)))
            (`SceneComponent.K2_AddWorldOffset` (`local.P`) (* (`KismetMathLibrary.MakeVector` -10.0) 10) false false)
            (`SceneComponent.K2_SetRelativeLocation` (`local.P_Mesh`) (50.0 0.0 0.0) false false)
            (`/Game/Blueprints/_Old/OldPlayer.Player_AddMovementInput` (`self.As Player`) (`local.P_Index`) (4.9 0.0 0.0) 1.0)))))))

(fn `TestCollide`
  (params (NewParam :type "/Game/Blueprints/Enums/E_Direction Enum" :default "NewEnumerator0") (P :type "BoxComponent Object Reference"))
  (returns (OutHit :type "HitResult Structure") (ReturnValue :type Boolean))
  (bind _returnvalue (`SceneComponent.GetForwardVector` P))
  (bind _returnvalue_2 (`SceneComponent.GetRightVector` P))
  (bind _returnvalue_3 (+ (`SceneComponent.K2_GetComponentLocation` P) (select `/Game/Blueprints/Enums/E_Direction` NewParam :`NewEnumerator0` (* _returnvalue_2 100) :`NewEnumerator1` (* _returnvalue_2 -100) :`NewEnumerator2` (* _returnvalue 100) :`NewEnumerator3` (* _returnvalue -100))))
  (bind (_outhit _returnvalue_4) (`KismetSystemLibrary.BoxTraceSingle` _returnvalue_3 _returnvalue_3 (45.0 45.0 45.0) (struct) "TraceTypeQuery1" false (`|MakeArray` (`self.GetOwner` P)) "ForOneFrame" true (struct :`R` 1.0 :`A` 1.0) (struct :`G` 1.0 :`A` 1.0) 0.1))
  (return _outhit _returnvalue_4))